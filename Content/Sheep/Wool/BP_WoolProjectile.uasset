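; BP_WoolProjectile is a wool projectile that deals damage to the actor it hits.
; When projectile movement stops, it sends a damage message to the hit actor and switches the Wool component to physics simulation with physics-only collision.
; If that message returns true, ChangeColor tints the wool to HitColor through a dynamic material instance created in the construction script.
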(event OnProjectileStop(ProjectileMovement)
  (params (ImpactResult :type Hit%20Result%20Structure%20%28by%20ref%29))
  (bind _wool (Variables|Default|GetWool))
  (bind _issuccessfull (Class|BPIHealth|TakeDamage(Message) (.HitActor (Collision|BreakHitResult ImpactResult)) 1.0))
  (Utilities|FlowControl|Sequence
    (:then_0
      (Physics|SetSimulatePhysics _wool true)
      (Collision|SetCollisionEnabled _wool "PhysicsOnly"))
    (:then_1
      (if _issuccessfull
        (CallFunction|ChangeColor (Variables|Default|GetHitColor))))))

(fn ConstructionScript
  (bind _returnvalue (Rendering|Material|CreateDynamicMaterialInstance (Rendering|Material|GetMaterial (Variables|Default|GetWool) 0) "None" "None" :!class /Script/Engine.KismetMaterialLibrary))
  (bind _output_get (Variables|Default|SetWoolMat _returnvalue))
  (Rendering|Material|SetMaterial (Variables|Default|GetWool) 0 _output_get))

(fn ChangeColor
  (params (NewColor :type Linear%20Color%20Structure))
  (Rendering|Material|SetVectorParameterValue (Variables|Default|GetWoolMat) (Variables|Default|GetParamName) NewColor :!class /Script/Engine.MaterialInstanceDynamic))