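; AC_Wool is an actor component that gives its owning BP_ThirdPersonCharacter a wool-projectile attack with limited ammo.
; On the attack input, it checks a cooldown timer and the remaining count, then spawns a BP_WoolProjectile ahead of the player and decrements the count.
; The last attack time starts at minus the cooldown so the first shot fires immediately, and debug prints report each attack or refusal.
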(event Input|EnhancedActionEvents|EnhancedInputActionIA_Attack
  (params (ActionValue :type Boolean) (ElapsedSeconds :type Float%20%28double-precision%29) (TriggeredSeconds :type Float%20%28double-precision%29) (InputAction :type Input%20Action%20Object%20Reference :default "/Game/ThirdPerson/Input/Actions/IA_Attack.IA_Attack"))
  (bind _returnvalue (CallFunction|ElapsedTime))
  (bind _count (Variables|Default|GetCount))
  (if (>= _returnvalue (Variables|Default|GetAttackCooldown))
    (if (> _count 0.0)
      (Development|PrintString "Attack")
      (Variables|Default|SetLast (Utilities|Time|GetGameTimeinSeconds))
      (Game|SpawnActorfromClass "/Game/Sheep/Wool/BP_WoolProjectile.BP_WoolProjectile_C" (CallFunction|SpawnTransform) "Undefined" "MultiplyWithRoot" 0 0)
      (Math|Float|DecrementFloat (Variables|Default|GetCount))
      (else
        (Development|PrintString (Utilities|String|Append "Not Enougth: " (Utilities|String|ToString(Float) _count)))))
    (else
      (Development|PrintString (Utilities|String|Append "Too Soon: " (Utilities|String|ToString(Float) _returnvalue))))))

(event EventBeginPlay
  (bind _asbp_third_person_character (Utilities|Casting|CastToBP_ThirdPersonCharacter (Components|GetOwner)))
  (Variables|Default|SetPlayer _asbp_third_person_character)
  (Variables|Default|SetLast (- 0.0 (Variables|Default|GetAttackCooldown))) ; Allow first attack
)

(fn ElapsedTime
  (return (- (Utilities|Time|GetGameTimeinSeconds) (Variables|Default|GetLast))))

(fn SpawnTransform
  (bind _player (Variables|Default|GetPlayer))
  (bind _returnvalue (Transformation|GetActorTransform _player))
  (return (Math|Transform|MakeTransform (+ (* (Transformation|GetActorForwardVector _player) (LocalVariables|GetForwardOffset)) (.location _returnvalue)) (.rotation _returnvalue))))