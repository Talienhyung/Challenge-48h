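; BP_Sheep is a wandering collectible sheep that rewards the third-person character with timer time, wool (Laine) and a sheep entry.
; On spawn it picks a weighted random material that sets its type, with rarer types generally paying more.
; It roams by re-calling an AI move to nearby random reachable points.
; On sphere overlap with the player, GetSheep derives the reward from the mesh material, then the sheep destroys itself.
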(event OnComponentBeginOverlap(Sphere)
  (params (OverlappedComponent :type Primitive%20Component%20Object%20Reference) (OtherActor :type Actor%20Object%20Reference) (OtherComp :type Primitive%20Component%20Object%20Reference) (OtherBodyIndex :type Integer) (bFromSweep :type Boolean) (SweepResult :type Hit%20Result%20Structure%20%28by%20ref%29))
  (bind _returnvalue (Actor|GetActorOfClass "/Game/ThirdPerson/Blueprints/BP_ThirdPersonCharacter.BP_ThirdPersonCharacter_C"))
  (if (== OtherActor _returnvalue)
    (Utilities|FlowControl|Delay 0.3)
    (bind (_name _pricetime _id _nbrlaine) (CallFunction|GetSheep))
    (Default|AddTimetoTimer _returnvalue _pricetime)
    (Default|AddLaine _returnvalue _nbrlaine)
    (Default|AddSheep _returnvalue _id _name)
    (Actor|DestroyActor)))

(event Custom|MoveSheep
  (bind _output_get (Variables|Default|SetRandom%20Location (.RandomLocation (AI|Navigation|GetRandomReachablePointinRadius (Transformation|GetActorLocation) 2e+02 0 0))))
  (AI|AIMoveTo self _output_get 0 3.0 true
    (:OnSuccess
      (Utilities|FlowControl|Delay 4.0)
      (CallFunction|MoveSheep))
    (:OnFail
      (Utilities|FlowControl|Delay 0.1)
      (CallFunction|MoveSheep))))

(event EventBeginPlay
  (bind _mesh (Variables|Character|GetMesh))
  (CallFunction|MoveSheep)
  (bind _newparam (CallFunction|RandomMaterial))
  (Rendering|Material|SetMaterial _mesh 0 _newparam)
  (Rendering|Material|SetMaterial _mesh 1 _newparam))

(fn ConstructionScript)

(fn MoveNPC)

(fn RandomMaterial
  (switch int (Math|Random|RandomIntegerinRange 0 19)
    (:Default
      _)
    (:0
      (return "/Game/StarterContent/Materials/M_CobbleStone_Rough.M_CobbleStone_Rough"))
    (:1
      (return "/Game/StarterContent/Materials/M_CobbleStone_Rough.M_CobbleStone_Rough"))
    (:2
      (return "/Game/StarterContent/Materials/M_CobbleStone_Rough.M_CobbleStone_Rough"))
    (:3
      (return "/Game/StarterContent/Materials/M_CobbleStone_Rough.M_CobbleStone_Rough"))
    (:4
      (return "/Game/StarterContent/Materials/M_CobbleStone_Rough.M_CobbleStone_Rough"))
    (:5
      (return "/Game/StarterContent/Props/Materials/M_Bush.M_Bush"))
    (:6
      (return "/Game/StarterContent/Props/Materials/M_Bush.M_Bush"))
    (:7
      (return "/Game/StarterContent/Props/Materials/M_Bush.M_Bush"))
    (:8
      (return "/Game/StarterContent/Props/Materials/M_Bush.M_Bush"))
    (:9
      (return "/Game/StarterContent/Props/Materials/M_Bush.M_Bush"))
    (:10
      (return "/Game/StarterContent/Props/Materials/M_Door.M_Door"))
    (:11
      (return "/Game/StarterContent/Props/Materials/M_Door.M_Door"))
    (:12
      (return "/Game/StarterContent/Props/Materials/M_Door.M_Door"))
    (:13
      (return "/Game/StarterContent/Props/Materials/M_Door.M_Door"))
    (:14
      (return "/Game/StarterContent/Blueprints/Assets/M_LightStage_Skybox_HDRI.M_LightStage_Skybox_HDRI"))
    (:15
      (return "/Game/StarterContent/Blueprints/Assets/M_LightStage_Skybox_HDRI.M_LightStage_Skybox_HDRI"))
    (:16
      (return "/Game/StarterContent/Blueprints/Assets/M_LightStage_Skybox_HDRI.M_LightStage_Skybox_HDRI"))
    (:17
      _)
    (:18
      _)
    (:19
      (return "/Game/LevelPrototyping/Materials/MI_Solid_Blue.MI_Solid_Blue")))
  (return "/Game/StarterContent/Materials/M_Metal_Gold.M_Metal_Gold"))

(fn GetSheep
  (bind _mesh (Variables|Character|GetMesh))
  (bind _returnvalue (Rendering|Material|GetMaterial _mesh 0))
  (if (== _returnvalue "/Game/StarterContent/Materials/M_Metal_Gold.M_Metal_Gold")
    _
    (elif (== _returnvalue "/Game/StarterContent/Materials/M_CobbleStone_Rough.M_CobbleStone_Rough")
      (return "Stone" 5.0 0 1)
      (elif (== _returnvalue "/Game/StarterContent/Props/Materials/M_Bush.M_Bush")
        (return "Bush" 5.0 1 1)
        (elif (== _returnvalue "/Game/StarterContent/Props/Materials/M_Door.M_Door")
          (return "Door" 1e+01 2 2)
          (elif (== _returnvalue "/Game/StarterContent/Blueprints/Assets/M_LightStage_Skybox_HDRI.M_LightStage_Skybox_HDRI")
            (return "Sky" 2e+01 3 3)
            (elif (== _returnvalue "/Game/LevelPrototyping/Materials/MI_Solid_Blue.MI_Solid_Blue")
              (return "Blue" 5e+01 5 8)
              (else
                _)))))))
  (return "Gold" 4e+01 4 4))