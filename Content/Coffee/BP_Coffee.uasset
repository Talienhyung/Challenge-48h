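; BP_Coffee is an enemy that chases the player and hits them for damage with knockback.
; A looping AI MoveTo drives an Idle, Walk and Attack state machine; success or failure returns to Idle and retries after a hit cooldown.
; Entering Attack damages the cached player health component and, if damage lands, launches the player away with an upward boost.
; ChangeState has stop and start hooks, but only Attack has logic.
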(event Custom|Move
  (bind _returnvalue (Game|GetPlayerCharacter 0))
  (Utilities|IsValid _returnvalue
    (:Is%20Valid
      (CallFunction|ChangeState "NewEnumerator1" false)
      (AI|AIMoveTo self "0, 0, 0" _returnvalue 0.0 false
        (:OnSuccess
          (CallFunction|ChangeState "NewEnumerator3" false))
        (:OnFail
          _))
      (CallFunction|ChangeState "NewEnumerator0" false)
      (Utilities|FlowControl|Delay (Variables|Default|GetHitCooldown))
      (CallFunction|Move))))

(event EventBeginPlay
  (CallFunction|ChangeState "NewEnumerator0" true)
  (CallFunction|Move)
  (bind _ac_health (CallFunction|GetPlayerHealthComponent))
  (Variables|Default|SetAC%20Health _ac_health)
  (bind _thirdpersoncharacter (CallFunction|GetThirdPersonCharacter))
  (Variables|Components|SetThird%20Person%20Character _thirdpersoncharacter))

(fn ConstructionScript)

(fn ChangeState
  (params (NewState :type E_CoffeeState%20Enum :default "NewEnumerator0") (FirstChange :type Boolean))
  (if (Utilities|Enum|NotEqual(Enum) NewState (Variables|Default|GetState))
    (Utilities|FlowControl|Sequence
      (:then_0
        ;[0.15 0.15 0.15 0.5] OnStop
        (switch Utilities|FlowControl|Switch|SwitchonE_CoffeeState (Variables|Default|GetState)))
      (:then_1
        (bind _output_get (Variables|Default|SetState NewState :!label _label))
        ;[0.15 0.15 0.15 0.5] OnStart
        (switch Utilities|FlowControl|Switch|SwitchonE_CoffeeState _output_get
          (:NewEnumerator3
            (bind _issuccessfull (Class|BPIHealth|TakeDamage(Message) (Variables|Default|GetAC%20Health) 1.0))
            (Development|PrintString (Utilities|String|SelectString "took damage" "didn't take damage" _issuccessfull))
            (if _issuccessfull
              (|Impulse))))))
    (elif FirstChange
      (goto _label))))